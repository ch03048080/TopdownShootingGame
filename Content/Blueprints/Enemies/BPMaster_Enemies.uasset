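; Master enemy Blueprint for forest monsters, handling health, attacks on the player and death.
; Spell hits subtract randomized damage and update a health widget with damage numbers and sound; the flashing hook is empty.
; A collision overlap gates delayed, Tick-driven touch damage and sphere-trace attacks between mesh sockets, with an ignore list preventing repeat hits.
; Death stops AI and collision, then drops a coin by monster type, increments the player's kill count and destroys the actor.
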(event `EnemyFlashingEffect`)

(event `self.ReceiveBeginPlay`
  (bind _aswbp_enemy_health (cast `/Game/Blueprints/Enemies/WBP_EnemyHealth` (`WidgetComponent.GetWidget` (`self.Widget`))))
  (set `self.As WBP Enemy Health` _aswbp_enemy_health)
  (set `self.Enemy Touch Damage` (- (`self.Enemy Damage`) 8.0)))

(event `self.ReceiveTick`
  (params (DeltaSeconds :type "Float (single-precision)"))
  (bind _overlapplayer (`self.OverlapPlayer`))
  ;[1 1 1] 몸통박치기
  (`KismetSystemLibrary.Delay` 0.5)
  (`/Engine/EditorBlueprintResources/StandardMacros.IsValid` _overlapplayer
    (:`Is Valid`
      (if (`self.IsAttack`)
        (`/Game/Blueprints/Player/BP_Player.Get Hurt and update health` _overlapplayer (`self.Enemy Touch Damage`))))))

(event `/Game/Blueprints/Enemies/BPI_Enemies.SpellCollisionEvent`
  (params (SpellDamageInput :type "Float (double-precision)"))
  (bind _returnvalue (`self.GetTransform`))
  (bind _charactermovement (`self.CharacterMovement`))
  (bind _returnvalue_2 (+ SpellDamageInput (`KismetMathLibrary.RandomFloatInRange` -5.0 5.0)))
  (bind _output_get (set `self.EnemyCurrentHealth` (- (`self.EnemyCurrentHealth`) _returnvalue_2)))
  (if (<= (`self.EnemyCurrentHealth`) 0.0)
    (`/Engine/EditorBlueprintResources/StandardMacros.DoOnce` false
      (:`Completed`
        ;[1 1 1] Enemy Die
        (`/Game/Blueprints/Enemies/WBP_EnemyHealth.UpdateEnemyHealthPercentage` (`self.As WBP Enemy Health`) 0.0)
        (`SkeletalMeshComponent.PlayAnimation` (`self.Mesh`) "/Game/UndeadPack/EnemyGoblin/Animations/Anim_Lose.Anim_Lose" false)
        (`BrainComponent.StopLogic` (`AIController.BrainComponent` (`AIBlueprintHelperLibrary.GetAIController` self)) "")
        (`PrimitiveComponent.SetCollisionEnabled` (`self.CapsuleComponent`) "NoCollision")
        (`PrimitiveComponent.SetCollisionEnabled` (`self.Mesh`) "NoCollision")
        (`/Engine/EditorBlueprintResources/StandardMacros.IsValid` _charactermovement
          (:`Is Valid`
            (`ActorComponent.K2_DestroyComponent` _charactermovement))
          (:`Is Not Valid`
            _))
        (`KismetSystemLibrary.Delay` 1.0)
        (switch `/Game/Blueprints/Enemies/E_ForestMonsterType` (`self.ForestMonsterType`)
          (:`NewEnumerator0`
            (`|SpawnActorFromClass` "/Game/Blueprints/Pickups/BP_Coin_Gold.BP_Coin_Gold_C" _returnvalue "Undefined" "OverrideRootScale" null null))
          (:`NewEnumerator1`
            (`|SpawnActorFromClass` "/Game/Blueprints/Pickups/BP_Coin_Silver.BP_Coin_Silver_C" _returnvalue "Undefined" "OverrideRootScale" null null))
          (:`NewEnumerator2`
            (`|SpawnActorFromClass` "/Game/Blueprints/Pickups/BP_Coin_Copper.BP_Coin_Copper_C" _returnvalue "Undefined" "OverrideRootScale" null null)))
        (bind _asbp_player (cast `/Game/Blueprints/Player/BP_Player` (`GameplayStatics.GetPlayerCharacter` 0)))
        (`/Game/Blueprints/Player/Widgets/WBP_Player.IncreaseKillCount` (`/Game/Blueprints/Player/BP_Player.Ref_Widget` _asbp_player))
        (`self.K2_DestroyActor`)))
    (else
      (`/Game/Blueprints/Enemies/WBP_EnemyHealth.UpdateEnemyHealthPercentage` (`self.As WBP Enemy Health`) (/ _output_get (`self.EnemyMaxHealth`)))
      (`GameplayStatics.PlaySoundAtLocation` "/Engine/EditorSounds/GamePreview/EjectFromPlayer_Cue.EjectFromPlayer_Cue" (`self.K2_GetActorLocation`) (struct) 1.0 1.0 0.0 null null null null)
      (`self.EnemyFlashingEffect`)
      (`/Game/Blueprints/Enemies/WBP_EnemyHealth.PlayDamageNumberAnimation` (`self.As WBP Enemy Health`) _returnvalue_2))))

(event `self.PlayerCollision.OnComponentBeginOverlap`
  (params (OverlappedComponent :type "PrimitiveComponent Object Reference") (OtherActor :type "Actor Object Reference") (OtherComp :type "PrimitiveComponent Object Reference") (OtherBodyIndex :type Integer) (bFromSweep :type Boolean) (SweepResult :type "HitResult Structure (by ref)"))
  (bind _asbp_player (cast `/Game/Blueprints/Player/BP_Player` OtherActor))
  (set `self.OverlapPlayer` _asbp_player)
  (set `self.IsAttack` true))

(event `self.PlayerCollision.OnComponentEndOverlap`
  (params (OverlappedComponent :type "PrimitiveComponent Object Reference") (OtherActor :type "Actor Object Reference") (OtherComp :type "PrimitiveComponent Object Reference") (OtherBodyIndex :type Integer))
  (cast `/Game/Blueprints/Player/BP_Player` OtherActor)
  (set `self.IsAttack` false))

(event `StartAttack`
  ;[1 1 1] Comment
  (bind _outhits (`KismetSystemLibrary.SphereTraceMultiForObjects` :`Start` (`SceneComponent.GetSocketLocation` (`self.Mesh`) (`self.Start`)) :`End` (`SceneComponent.GetSocketLocation` (`self.Mesh`) (`self.End`)) :`Radius` 100.0 :`ObjectTypes` (`|MakeArray` "ObjectTypeQuery3" :!type "EObjectTypeQuery Enum") :`DrawDebugType` "ForDuration"))
  (for _array_element _outhits
    (bind (_bblockinghit _binitialoverlap _time _distance _location _impactpoint _normal _impactnormal _physmat _hitactor) (`GameplayStatics.BreakHitResult` _array_element))
    (if (not (`KismetArrayLibrary.Array_Contains` (`self.actorignore`) _hitactor))
      (bind _asbp_player (cast `/Game/Blueprints/Player/BP_Player` _hitactor))
      (if (`self.IsAttack`)
        (`/Game/Blueprints/Player/BP_Player.Get Hurt and update health` _asbp_player (`self.Enemy Damage`)))
      (`KismetArrayLibrary.Array_Add` (`self.actorignore`) _hitactor)))
  (`KismetSystemLibrary.Delay` 0.2))

(event `EndAttack`
  ;[1 1 1] Comment
  (`KismetArrayLibrary.Array_Clear` (`self.Actorignore`)))

(fn `UserConstructionScript`)