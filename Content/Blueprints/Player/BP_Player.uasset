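; Player character for a top-down auto-spell survival game, moved by Enhanced Input and turned toward the cursor.
; BeginPlay creates the HUD, enemy spawner and timers; coin XP triggers a paused skill-selection screen, and zero health a death screen.
; Five-level spells use rotated pivots: fireballs fan out, ice balls form randomly oriented rings, and light orbs orbit on a looping Timeline.
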(event `LightBallSpell`
  (bind _outactors (`GameplayStatics.GetAllActorsOfClass` "/Game/Blueprints/Player/Spells/Spell_Light_Straight.Spell_Light_Straight_C"))
  (for _array_element _outactors
    (`self.K2_DestroyActor` _array_element))
  (switch `int` (`self.SpellLevel_Light`)
    (:`1`
      (`self.Initialize Light Spell` 3 120.0))
    (:`2`
      (`self.Initialize Light Spell` 4 90.0))
    (:`3`
      (`self.Initialize Light Spell` 5 72.0))
    (:`4`
      (`self.Initialize Light Spell` 6 60.0))
    (:`5`
      (`self.Initialize Light Spell` 8 45.0))))

(event `IceSpell`
  ;[1 1 1] Ice
  (switch `int` (`self.SpellLevel_Ice`)
    (:`1`
      (`self.SpellSpawnIceBalls` 3 0.0 120.0))
    (:`2`
      (`self.SpellSpawnIceBalls` 4 0.0 90.0))
    (:`3`
      (`self.SpellSpawnIceBalls` 5 0.0 72.0))
    (:`4`
      (`self.SpellSpawnIceBalls` 6 0.0 60.0))
    (:`5`
      (`self.SpellSpawnIceBalls` 8 0.0 45.0))))

(event `Fireball`
  ;[1 0.08333 0.08333] Fire
  (switch `int` (`self.SpellLevel_Fire`)
    (:`1`
      (`self.SpellSpawnFireballs` 1))
    (:`2`
      (`self.SpellSpawnFireballs` 2 -10.0 20.0))
    (:`3`
      (`self.SpellSpawnFireballs` 3 -15.0 15.0))
    (:`4`
      (`self.SpellSpawnFireballs` 4 -15.0 10.0))
    (:`5`
      (`self.SpellSpawnFireballs` 5 -20.0 10.0))))

(event `Initialize Light Spell`
  (params (NumOfOrbs :type Integer) (OrbRotation :type "Float (double-precision)"))
  (bind _lightorbspawn (`self.LightOrbSpawn`))
  (for _ (range 1 (+ NumOfOrbs 1))
    (bind _returnvalue (`|SpawnActorFromClass` "/Game/Blueprints/Player/Spells/Spell_Light_Straight.Spell_Light_Straight_C" (`KismetMathLibrary.MakeTransform` (`SceneComponent.K2_GetComponentLocation` _lightorbspawn) (`SceneComponent.K2_GetComponentRotation` _lightorbspawn)) "Undefined" "OverrideRootScale" null null))
    (`self.K2_AttachToComponent` _returnvalue (`self.LightOrbRotatingPivot`) "None" "KeepWorld" "KeepWorld" "KeepWorld" true)
    (`SceneComponent.K2_AddLocalRotation` (`self.LightOrbPivot`) (`KismetMathLibrary.MakeRotator` 0.0 0.0 OrbRotation) false false)))

(event `Start Ice Spell`
  ;[1 1 1] Ice
  (`KismetSystemLibrary.K2_SetTimerDelegate` (`|CreateDelegate` :!event `IceSpell`) 1.5 true))

(event `StartRotatingLight`
  (bind (_direction _newtrack_0) (`Timeline|Timeline` :!via `PlayFromStart`)
    (:`Update`
      (`SceneComponent.K2_SetRelativeRotation` (`self.LightOrbRotatingPivot`) (`KismetMathLibrary.MakeRotator` 0.0 0.0 (`KismetMathLibrary.Lerp` 0.0 360.0 _newtrack_0)) false false))
    (:`Finished`
      (`self.StartRotatingLight`))))

(event `self.ReceiveBeginPlay`
  ;[1 1 1] Comment
  (`EnhancedInputSubsystemInterface.AddMappingContext` (pcsubsystem `EnhancedInputLocalPlayerSubsystem` (`GameplayStatics.GetPlayerController` 0)) "/Game/Blueprints/Player/IMC_Player.IMC_Player" 0 (struct))
  (bind _returnvalue (`|CreateWidget` "/Game/Blueprints/Player/Widgets/WBP_Player.WBP_Player_C"))
  (bind _output_get (set `self.Ref_Widget` _returnvalue))
  (`UserWidget.AddToViewport` _output_get 0)
  (`KismetSystemLibrary.K2_SetTimerDelegate` (`|CreateDelegate` :!event `Fireball`) 1.0 true)
  (bind _returnvalue_2 (`|SpawnActorFromClass` "/Game/Blueprints/Player/BP_EnemySpawn.BP_EnemySpawn_C" (`KismetMathLibrary.MakeTransform` (`self.K2_GetActorLocation`)) "Undefined" "OverrideRootScale" null null))
  (set `self.Ref_Spawner` _returnvalue_2)
  (`KismetSystemLibrary.K2_SetTimerDelegate` (`|CreateDelegate` :!event `UpdateTimer`) 1.0 true))

(event `AddCoinExperience`
  (params (PickupValue :type "Float (double-precision)"))
  ;[1 1 1] XP
  (set `self.CurrentExperience` (+ (`self.CurrentExperience`) PickupValue))
  (`/Game/Blueprints/Player/Widgets/WBP_Player.UpdateXP_Percentage` (`self.Ref_Widget`) (/ (`self.CurrentExperience`) (`self.ExperienceCap`)))
  (if (>= (`self.CurrentExperience`) (`self.ExperienceCap`))
    (`/Game/Blueprints/Player/Widgets/WBP_Player.UpdateXP_Percentage` (`self.Ref_Widget`) 0.0)
    (`/Engine/EditorBlueprintResources/StandardMacros.IncrementInt` (`self.CharacterLevel`)
      (:`  `
        (set `self.CurrentExperience` 0.0)
        (`self.StartSelectingSkills`)
        (`/Game/Blueprints/Player/Widgets/WBP_Player.IncreaseLevel` (`self.Ref_Widget`) (`self.CharacterLevel`))))))

(event `StartSelectingSkills`
  ;[1 1 1] SkillSelect
  (`self.SkillLevelupFunction` true true)
  (`WidgetBlueprintLibrary.SetInputMode_UIOnlyEx` (`GameplayStatics.GetPlayerController` 0) (`self.Ref_Widget`)))

(event `ReturnToGame`
  ;[1 1 1] SkillSelect
  (`self.SkillLevelupFunction` false false "MOVE_Walking" "Hidden")
  (`WidgetBlueprintLibrary.SetInputMode_GameOnly` (`GameplayStatics.GetPlayerController` 0)))

(event `EnhancedInput|/Game/Blueprints/Player/IA_Movement`
  (params (ActionValue :type "Vector2D Structure") (ElapsedSeconds :type "Float (double-precision)") (TriggeredSeconds :type "Float (double-precision)") (InputAction :type "InputAction Object Reference" :default "/Game/Blueprints/Player/IA_Movement.IA_Movement"))
  ;[1 1 1] Movement
  (:`Triggered`
    (`self.AddMovementInput` (1.0 0.0 0.0) ActionValue_X)
    (`self.AddMovementInput` (0.0 1.0 0.0) ActionValue_Y)))

(event `UpdateTimer`
  ;[1 1 1] TimerHUD
  (`/Engine/EditorBlueprintResources/StandardMacros.IncrementInt` (`self.Seconds`)
    (:`  `
      (if (== (`self.Seconds`) 60)
        (`/Engine/EditorBlueprintResources/StandardMacros.IncrementInt` (`self.Minutes`)
          (:`  `
            (set `self.Seconds` 0))))
      (`/Game/Blueprints/Player/Widgets/WBP_Player.UpdateTimer` (`self.Ref_Widget`) (`self.Minutes`) (`self.Seconds`)))))

(event `Get Hurt and update health`
  (params (EnemyDamage :type "Float (double-precision)"))
  (bind _returnvalue (`GameplayStatics.GetPlayerController` 0))
  (bind _wbp_deathscreen (`/Game/Blueprints/Player/Widgets/WBP_Player.WBP_DeathScreen` (`self.Ref_Widget`)))
  ;[1 1 1] Health
  (bind _output_get (set `self.Player_Health` (- (`self.Player_Health`) EnemyDamage)))
  (`/Game/Blueprints/Player/Widgets/WBP_Player.UpdatePercentage` (`self.Ref_Widget`) (/ _output_get (`self.Player_MaxHealth`)))
  (if (<= (`self.Player_Health`) 0.0)
    (`GameplayStatics.SetGamePaused` true)
    (`Widget.SetVisibility` _wbp_deathscreen "Visible")
    (`/Game/Blueprints/Player/Widgets/WBP_DeathScreen.playFadeAnimation` _wbp_deathscreen)
    (`WidgetBlueprintLibrary.SetInputMode_UIOnlyEx` _returnvalue null)
    (set `PlayerController.bShowMouseCursor` true _returnvalue)))

(event `TopRightHUD_Fire`
  ;[1 1 1] TopRightHUD
  (`/Game/Blueprints/Player/Widgets/WBP_TopRightHUD.UpdateFire` (`/Game/Blueprints/Player/Widgets/WBP_Player.WBP_TopRight` (`self.Ref_Widget`)) (`self.SpellLevel_Fire`)))

(event `TopRightHUD_Ice`
  ;[1 1 1] TopRightHUD
  (`/Game/Blueprints/Player/Widgets/WBP_TopRightHUD.UpdateIce` (`/Game/Blueprints/Player/Widgets/WBP_Player.WBP_TopRight` (`self.Ref_Widget`)) (`self.SpellLevel_Ice`)))

(event `TopRightHUD_Light`
  ;[1 1 1] TopRightHUD
  (`/Game/Blueprints/Player/Widgets/WBP_TopRightHUD.UpdateLight` (`/Game/Blueprints/Player/Widgets/WBP_Player.WBP_TopRight` (`self.Ref_Widget`)) (`self.SpellLevel_Light`)))

(event `self.ReceiveTick`
  (params (DeltaSeconds :type "Float (single-precision)"))
  (bind (_returnvalue_x _returnvalue_y) (`KismetMathLibrary.BreakVector` (`self.K2_GetActorLocation`)))
  (bind (_bblockinghit _binitialoverlap _time _distance _location) (`GameplayStatics.BreakHitResult` (`PlayerController.GetHitResultUnderCursorByChannel` (`GameplayStatics.GetPlayerController` 0) "TraceTypeQuery1" true)))
  ;[1 1 1] Comment
  (`self.K2_SetActorRotation` (`KismetMathLibrary.FindLookAtRotation` (`KismetMathLibrary.MakeVector` _returnvalue_x _returnvalue_y) (`KismetMathLibrary.MakeVector` (.x _location) (.y _location))))
  (`SceneComponent.K2_SetWorldLocation` (`self.Sphere`) (`KismetMathLibrary.MakeVector` (.x _location) (.y _location)) false false))

(event `TopRightHUD_Dark`
  ;[1 1 1] TopRightHUD
  (`/Game/Blueprints/Player/Widgets/WBP_TopRightHUD.UpdateDark` (`/Game/Blueprints/Player/Widgets/WBP_Player.WBP_TopRight` (`self.Ref_Widget`)) (`self.SpellLevel_Dark`)))

(fn `SkillLevelupFunction`
  (params (bPaused :type Boolean) (`Show Mouse Cursor` :type Boolean) (NewMovementMode :type "EMovementMode Enum" :default "MOVE_None") (InVisibility :type "ESlateVisibility Enum" :default "Visible"))
  (`GameplayStatics.SetGamePaused` bPaused)
  (set `PlayerController.bShowMouseCursor` `Show Mouse Cursor` (`GameplayStatics.GetPlayerController` 0))
  (`CharacterMovementComponent.SetMovementMode` (`self.CharacterMovement`) NewMovementMode 0)
  (`Widget.SetVisibility` (`/Game/Blueprints/Player/Widgets/WBP_Player.WBP_Leveling` (`self.Ref_Widget`)) InVisibility)
  (return))

(fn `SpellSpawnFireballs`
  (params (NumberOfProjectiles :type Integer) (`Start Rotation` :type "Float (double-precision)") (`Rotation Increment` :type "Float (double-precision)"))
  (bind _fireballspawn (`self.FireBallSpawn`))
  (`SceneComponent.K2_SetRelativeRotation` (`self.FireBallPivot`) (`KismetMathLibrary.MakeRotator` 0.0 0.0 `Start Rotation`) false false)
  (for _ (range 1 (+ NumberOfProjectiles 1))
    (`|SpawnActorFromClass` "/Game/Blueprints/Player/Spells/Spell_Fire.Spell_Fire_C" (`KismetMathLibrary.MakeTransform` (`SceneComponent.K2_GetComponentLocation` _fireballspawn) (`SceneComponent.K2_GetComponentRotation` _fireballspawn)) "Undefined" "OverrideRootScale" null null)
    (`SceneComponent.K2_AddRelativeRotation` (`self.FireBallPivot`) (`KismetMathLibrary.MakeRotator` 0.0 0.0 `Rotation Increment`) false false))
  (`SceneComponent.K2_SetRelativeRotation` :`self` (`self.FireBallPivot`)))

(fn `SpellSpawnIceBalls`
  (params (NumberOfProjectiles :type Integer) (`Start Rotation` :type "Float (double-precision)") (`Rotation Increment` :type "Float (double-precision)"))
  (bind _iceballspawn (`self.IceBallSpawn`))
  (`SceneComponent.K2_SetRelativeRotation` (`self.IceBallPivot`) (`KismetMathLibrary.MakeRotator` 0.0 0.0 (`KismetMathLibrary.RandomFloatInRange` 0.0 360.0)) false false)
  (for _ (range 1 (+ NumberOfProjectiles 1))
    (`|SpawnActorFromClass` "/Game/Blueprints/Player/Spells/Spell_Ice.Spell_Ice_C" (`KismetMathLibrary.MakeTransform` (`SceneComponent.K2_GetComponentLocation` _iceballspawn) (`SceneComponent.K2_GetComponentRotation` _iceballspawn)) "Undefined" "OverrideRootScale" null null)
    (`SceneComponent.K2_AddRelativeRotation` (`self.IceBallPivot`) (`KismetMathLibrary.MakeRotator` 0.0 0.0 `Rotation Increment`) false false))
  (`SceneComponent.K2_SetRelativeRotation` :`self` (`self.IceBallPivot`)))

(fn `UserConstructionScript`)